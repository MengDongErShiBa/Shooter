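; Enemy Blueprint that handles the enemy's health bar and floating damage numbers.
; On BeginPlay it links the health bar widget to itself and hides it, then show and hide events toggle its visibility, with show also calling the parent implementation.
; Each hit spawns a number widget at the screen-projected hit location, sets its damage text and headshot flag, plays its animation, and passes it to StoreHitNumber.
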(event `self.ReceiveBeginPlay`
  (bind _returnvalue (`WidgetComponent.GetUserWidgetObject` (`self.HealthBar`)))
  (bind _asenemy_health_bar (cast `/Game/_Game/HUD/EnemyHealthBar` _returnvalue))
  (set `/Game/_Game/HUD/EnemyHealthBar.Enemy` self _asenemy_health_bar)
  (`Widget.SetVisibility` _returnvalue "Hidden"))

(event `self.ShowHealthBar`
  (set `Widget.Visibility` "Visible" (`WidgetComponent.GetUserWidgetObject` (`self.HealthBar`)))
  (`parent.ShowHealthBar`))

(event `self.HideHealthBar`
  (set `Widget.Visibility` "Hidden" (`WidgetComponent.GetUserWidgetObject` (`self.HealthBar`))))

(event `self.ShowHitNumber`
  (params (Damage :type Integer) (HitLocation :type "Vector Structure") (bHeadShot :type Boolean))
  (bind _returnvalue (`|CreateWidget` "/Game/_Game/HUD/HItNumber.HItNumber_C"))
  (`self.StoreHitNumber` _returnvalue HitLocation)
  (`UserWidget.SetPositionInViewport` _returnvalue (`WidgetLayoutLibrary.ProjectWorldLocationToWidgetPosition` (`GameplayStatics.GetPlayerController` 0) HitLocation true) false)
  (`UserWidget.AddToViewport` _returnvalue 0)
  (set `/Game/_Game/HUD/HItNumber.HitText` (`KismetTextLibrary.Conv_IntToText` Damage) _returnvalue)
  (set `/Game/_Game/HUD/HItNumber.HeadShot` bHeadShot _returnvalue)
  (`UserWidget.PlayAnimation` _returnvalue (`/Game/_Game/HUD/HItNumber.HitNumberAnimation` _returnvalue) 0.0 1 "Forward" 1.0 false))

(fn `UserConstructionScript`)