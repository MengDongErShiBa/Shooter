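; Shooter HUD that draws a dynamic, weapon-specific crosshair at the center of the screen.
; BeginPlay caches the player's ShooterCharacterBP, and DrawHUD re-acquires it whenever the reference is invalid.
; Each draw reads the character's crosshair spread multiplier, scaled by a maximum spread to push the top, bottom, left and right textures outward.
; These four textures and a fixed middle one come from the equipped weapon.
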(event `self.ReceiveBeginPlay`
  ;[1 1 1] 获取角色引用
  (`/Engine/EditorBlueprintResources/StandardMacros.IsValid` (`self.ShooterCharacter`)
    (:`Is Not Valid`
      (bind _asshooter_character_bp (cast `/Game/_Game/Character/ShooterCharacterBP` (`GameplayStatics.GetPlayerPawn` 0)))
      (set `self.ShooterCharacter` _asshooter_character_bp))))

(event `self.ReceiveDrawHUD`
  (params (SizeX :type Integer) (SizeY :type Integer))
  (bind (_x _y) (`KismetMathLibrary.BreakVector2D` (`self.CrosshairBaseCenter`)))
  (bind (_x_2 _y_2) (`KismetMathLibrary.BreakVector2D` (`self.CrosshairBaseCenter`)))
  (bind (_x_3 _y_3) (`KismetMathLibrary.BreakVector2D` (`self.CrosshairBaseCenter`)))
  (bind (_x_4 _y_4) (`KismetMathLibrary.BreakVector2D` (`self.CrosshairBaseCenter`)))
  (bind (_x_5 _y_5) (`KismetMathLibrary.BreakVector2D` (`self.CrosshairBaseCenter`)))
  (bind (_x_6 _y_6) (`KismetMathLibrary.BreakVector2D` (`self.CrosshairLocation`)))
  (bind (_x_7 _y_7) (`KismetMathLibrary.BreakVector2D` (`self.ScreenCenter`)))
  ;[1 1 1] 设置屏幕中心和准心位置
  (set `self.ScreenCenter` (`KismetMathLibrary.MakeVector2D` (`KismetMathLibrary.Conv_IntToDouble` (/ SizeX 2)) (`KismetMathLibrary.Conv_IntToDouble` (/ SizeY 2))))
  (set `self.CrosshairLocation` (`KismetMathLibrary.MakeVector2D` _x_7 _y_7))
  ;[1 1 1] 确认ShooterCcharacter有效
  (`/Engine/EditorBlueprintResources/StandardMacros.IsValid` (`self.ShooterCharacter`)
    (:`Is Valid`
      _)
    (:`Is Not Valid`
      (bind _asshooter_character_bp (cast `/Game/_Game/Character/ShooterCharacterBP` (`GameplayStatics.GetPlayerPawn` 0)))
      (set `self.ShooterCharacter` _asshooter_character_bp)))
  ;[1 1 1] 获得准心扩散系数
  (set `self.CrosshairSpreadMultiplier` (`ShooterCharacter.GetCrosshairSpreadMultiplier` (`self.ShooterCharacter`)))
  ;[1 1 1] 准心中心位置
  (set `self.CrosshairBaseCenter` (`KismetMathLibrary.MakeVector2D` (- _x_6 (`self.CrosshairHalfWidth`)) (- _y_6 (`self.CrosshairHalfHeight`))))
  (`self.DrawTexture` (`Weapon.CrosshairBottom` (`ShooterCharacter.EquippedWeapon` (`self.ShooterCharacter`))) _x_2 (+ _y_2 (* (`self.CrosshairSpreadMultiplier`) (`self.CrosshairSpreadMax`))) 64.0 64.0 0.0 0.0 1.0 1.0)
  (`self.DrawTexture` (`Weapon.CrosshairTop` (`ShooterCharacter.EquippedWeapon` (`self.ShooterCharacter`))) _x_3 (- _y_3 (* (`self.CrosshairSpreadMultiplier`) (`self.CrosshairSpreadMax`))) 64.0 64.0 0.0 0.0 1.0 1.0)
  (`self.DrawTexture` (`Weapon.CrosshairLeft` (`ShooterCharacter.EquippedWeapon` (`self.ShooterCharacter`))) (- _x_4 (* (`self.CrosshairSpreadMultiplier`) (`self.CrosshairSpreadMax`))) _y_4 64.0 64.0 0.0 0.0 1.0 1.0)
  (`self.DrawTexture` (`Weapon.CrosshairRight` (`ShooterCharacter.EquippedWeapon` (`self.ShooterCharacter`))) (+ _x_5 (* (`self.CrosshairSpreadMultiplier`) (`self.CrosshairSpreadMax`))) _y_5 64.0 64.0 0.0 0.0 1.0 1.0)
  (`self.DrawTexture` (`Weapon.CrosshairMiddle` (`ShooterCharacter.EquippedWeapon` (`self.ShooterCharacter`))) _x _y 64.0 64.0 0.0 0.0 1.0 1.0))

(fn `UserConstructionScript`)